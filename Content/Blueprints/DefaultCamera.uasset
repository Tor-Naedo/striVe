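; Shared two-player camera that follows both players on the Y and Z axes while keeping its own X position.
; After a short BeginPlay delay, it gets both players from DefaultGameModeBP and spawns two BoundariesCam actors, placed once beyond each player along Y as left and right edges.
; Each Tick it moves near the players' midpoint, using divisors slightly under two, and scales field of view with their Y separation within a clamped range.
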(event EventBeginPlay
  (Utilities|FlowControl|Delay 0.03)
  (bind _asdefault_game_mode_bp (Utilities|Casting|CastToDefaultGameModeBP (Game|GetGameMode)))
  (Utilities|IsValid (Variables|/Script/striVe.striVeGameMode|Getplayer1 _asdefault_game_mode_bp)
    (:Is%20Valid
      (Variables|Default|SetPlayer1Ref (Variables|/Script/striVe.striVeGameMode|Getplayer1 _asdefault_game_mode_bp))
      (Utilities|IsValid (Variables|/Script/striVe.striVeGameMode|Getplayer2 _asdefault_game_mode_bp)
        (:Is%20Valid
          (Variables|Default|SetPlayer2Ref (Variables|/Script/striVe.striVeGameMode|Getplayer2 _asdefault_game_mode_bp))
          (bind _returnvalue (Game|SpawnActorfromClass "/Game/Blueprints/BoundariesCam.BoundariesCam_C" (Transformation|GetActorTransform) "Undefined" 0 0))
          (Variables|Default|SetLeftCameraEdge _returnvalue)
          (bind _returnvalue_2 (Game|SpawnActorfromClass "/Game/Blueprints/BoundariesCam.BoundariesCam_C" (Transformation|GetActorTransform) "Undefined" 0 0))
          (Variables|Default|SetRightCameraEdge _returnvalue_2)
          (CallFunction|SetCameraBoundaries))))))

(event EventTick
  (params (DeltaSeconds :type Float%20%28single-precision%29))
  (bind _player1ref (Variables|Default|GetPlayer1Ref))
  (bind _player2ref (Variables|Default|GetPlayer2Ref))
  (bind _returnvalue (Transformation|GetActorLocation _player1ref))
  (bind _returnvalue_2 (Transformation|GetActorLocation _player2ref))
  (bind (_x _y _z) (Math|Vector|BreakVector _returnvalue))
  (bind (_x_2 _y_2 _z_2) (Math|Vector|BreakVector _returnvalue_2))
  (if (and (Utilities|IsValid _player1ref) (Utilities|IsValid _player2ref))
    (Transformation|SetActorLocation (Math|Vector|MakeVector (.X (Math|Vector|BreakVector (Transformation|GetActorLocation))) (/ (+ _y _y_2) 1.9) (/ (+ _z_2 _z) 1.7)) false false)
    (Camera|SetFieldOfView (Variables|CameraActor|GetCameraComponent) (Math|Float|Clamp(Float) (Math|Float|Absolute(Float) (* (- (.Y (Math|Vector|BreakVector (Transformation|GetActorLocation (Variables|Default|GetPlayer1Ref)))) (.Y (Math|Vector|BreakVector (Transformation|GetActorLocation (Variables|Default|GetPlayer2Ref))))) 0.15)) 6e+01 8e+01))))

(fn ConstructionScript)

(fn SetCameraBoundaries
  (bind _player1ref (Variables|Default|GetPlayer1Ref))
  (bind _player2ref (Variables|Default|GetPlayer2Ref))
  (bind _returnvalue (Transformation|GetActorLocation _player2ref))
  (bind _returnvalue_2 (Transformation|GetActorLocation _player1ref))
  (bind (_x _y _z) (Math|Vector|BreakVector _returnvalue))
  (bind (_x_2 _y_2 _z_2) (Math|Vector|BreakVector _returnvalue_2))
  (Transformation|SetActorLocation (Variables|Default|GetLeftCameraEdge) (Math|Vector|MakeVector _x_2 (- _y_2 5e+02) _z_2) false false)
  (Transformation|SetActorLocation (Variables|Default|GetRightCameraEdge) (Math|Vector|MakeVector _x (+ _y 5e+02) _z) false false))