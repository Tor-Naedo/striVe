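; Base character Blueprint for striVe that sets up a hurtbox and lets a second player share the keyboard.
; After a short delay on BeginPlay, it caches the game mode's Player2 unless that is itself, then spawns and attaches an owned HurtboxBP.
; P2 jump, attack and move inputs received here are forwarded to Player2's P2Keyboard functions, with debug prints left in.
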(event EventBeginPlay
  (bind _self self)
  (Utilities|FlowControl|Delay 0.2)
  (bind _asstri_ve_game_mode (Utilities|Casting|CastTostriVeGameMode (Game|GetGameMode)))
  (bind _output_get (Variables|Default|SetGameModeReference _asstri_ve_game_mode))
  (if (== (Variables|/Script/striVe.striVeGameMode|Getplayer2 _output_get) self)
    _
    (else
      (Variables|Default|SetPlayer2Reference (Variables|/Script/striVe.striVeGameMode|Getplayer2 _output_get))))
  (bind _returnvalue (Game|SpawnActorfromClass "/Game/Blueprints/HurtboxBP.HurtboxBP_C" (Transformation|GetActorTransform (Class|CharacterMovementComponent|GetCharacterOwner (Variables|Character|GetCharacterMovement))) "Undefined" 0 0))
  (bind _output_get_2 (Variables|Default|Sethurtbox _returnvalue))
  (Transformation|AttachActorToActor _output_get_2 _self "None" "SnapToTarget" "SnapToTarget" "SnapToTarget" true)
  (Actor|SetOwner _returnvalue _self))

(event EventTick
  (params (DeltaSeconds :type Float%20%28single-precision%29)))

(event Input|ActionEvents|InputActionJumpP2
  (params (Key :type Key%20Structure :default "None"))
  (bind _player2reference (Variables|Default|GetPlayer2Reference))
  (bind _player2reference_2 (Variables|Default|GetPlayer2Reference))
  (:Pressed
    (Utilities|IsValid _player2reference
      (:Is%20Valid
        (Class|StriVeCharacter|P2KeyboardJump _player2reference)
        (Development|PrintString "Hello"))))
  (:Released
    (Utilities|IsValid _player2reference_2
      (:Is%20Valid
        (Class|StriVeCharacter|P2KeyboardStopJumping _player2reference_2)
        (Development|PrintString "Hello")))))

(event Input|ActionEvents|InputActionAttack1P2
  (params (Key :type Key%20Structure :default "None"))
  (bind _player2reference (Variables|Default|GetPlayer2Reference))
  (:Pressed
    (Utilities|IsValid _player2reference
      (:Is%20Valid
        (Class|StriVeCharacter|P2KeyboardAttack1 _player2reference)
        (Development|PrintString "Hello"))
      (:Is%20Not%20Valid
        (Development|PrintString "not valid")))))

(event Input|ActionEvents|InputActionAttack2P2
  (params (Key :type Key%20Structure :default "None"))
  (bind _player2reference (Variables|Default|GetPlayer2Reference))
  (:Pressed
    (Utilities|IsValid _player2reference
      (:Is%20Valid
        (Class|StriVeCharacter|P2KeyboardAttack2 _player2reference)
        (Development|PrintString "Hello")))))

(event Input|ActionEvents|InputActionAttack3P2
  (params (Key :type Key%20Structure :default "None"))
  (bind _player2reference (Variables|Default|GetPlayer2Reference))
  (:Pressed
    (Utilities|IsValid _player2reference
      (:Is%20Valid
        (Class|StriVeCharacter|P2KeyboardAttack3 _player2reference)
        (Development|PrintString "Hello")))))

(event Input|ActionEvents|InputActionAttack4P2
  (params (Key :type Key%20Structure :default "None"))
  (bind _player2reference (Variables|Default|GetPlayer2Reference))
  (:Pressed
    (Utilities|IsValid _player2reference
      (:Is%20Valid
        (Class|StriVeCharacter|P2KeyboardAttack4 _player2reference)
        (Development|PrintString "Hello")))))

(event Input|AxisEvents|InputAxisMoveRightP2
  (params (AxisValue :type Float%20%28single-precision%29))
  (bind _player2reference (Variables|Default|GetPlayer2Reference))
  (Utilities|IsValid _player2reference
    (:Is%20Valid
      (Class|StriVeCharacter|P2KeyboardMoveRight _player2reference AxisValue)
      (Development|PrintString "Hello"))))

(fn ConstructionScript)