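; Hitbox actor for a two-player fighting game that applies damage to the opposing player.
; SpawnHitbox sets the display material by hitbox type (Proximity, Strike or Hurtbox), moves the mesh to HitboxLocation, hides it and checks collision.
; CheckCollision uses the striVeGameMode player references to identify the owner, then damages the opponent if overlapping their hurtbox.
; The overlap is tested once per spawn call, regardless of hitbox type.
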(event Custom|SpawnHitbox
  (switch Utilities|FlowControl|Switch|SwitchonEHitboxEnum (Variables|Default|GethitboxType)
    (:HB_PROXIMITY
      (Rendering|Material|SetMaterial (Variables|Default|GetHitboxDisplay) 0 "/Game/Art/Materials/Hitboxes/M_ProximityHitbox.M_ProximityHitbox"))
    (:HB_STRIKE
      (Rendering|Material|SetMaterial (Variables|Default|GetHitboxDisplay) 0 "/Game/Art/Materials/Hitboxes/M_StrikeHitbox.M_StrikeHitbox"))
    (:HB_HURTBOX
      (Rendering|Material|SetMaterial (Variables|Default|GetHitboxDisplay) 0 "/Game/Art/Materials/Hitboxes/M_Hurtbox.M_Hurtbox")))
  (Transformation|SetWorldLocation (Variables|Default|GetHitboxDisplay) (Variables|Default|GethitboxLocation) false false)
  (Rendering|SetVisibility (Variables|Default|GetHitboxDisplay) false false)
  (CallFunction|CheckCollision))

(event Custom|CheckCollision
  (bind _basegamemodereference (Variables|Default|GetBaseGameModeReference))
  (bind _basegamemodereference_2 (Variables|Default|GetBaseGameModeReference))
  (bind _player1 (Variables|/Script/striVe.striVeGameMode|Getplayer1 _basegamemodereference))
  (bind _player2 (Variables|/Script/striVe.striVeGameMode|Getplayer2 _basegamemodereference_2))
  (bind _isplayerone (CallFunction|DeterminePlayer))
  (if _isplayerone
    (if (Collision|IsOverlappingActor (Variables|/Script/striVe.striVeCharacter|Gethurtbox _player2) :!class /Script/Engine.Actor)
      (Class|StriVeCharacter|TakeDamage _player2 (Variables|Default|GethitboxDamage)))
    (elif (Collision|IsOverlappingActor (Variables|/Script/striVe.striVeCharacter|Gethurtbox _player1) :!class /Script/Engine.Actor)
      (Class|StriVeCharacter|TakeDamage _player1 (Variables|Default|GethitboxDamage)))))

(fn ConstructionScript)

(fn DeterminePlayer
  (bind _asstri_ve_game_mode (Utilities|Casting|CastTostriVeGameMode (Game|GetGameMode)))
  (bind _output_get (Variables|Default|SetBaseGameModeReference _asstri_ve_game_mode))
  (if (== (Variables|/Script/striVe.striVeGameMode|Getplayer1 _output_get) (Components|GetOwner))
    (return true)
    (else
      (return false))))