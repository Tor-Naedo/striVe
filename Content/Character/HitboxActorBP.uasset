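; Hitbox actor for character combat that shows a colored box and damages the player character on overlap.
; SpawnHitbox picks the display material by hitbox type (proximity, strike or hurtbox), then moves the display to the hitbox location and makes it visible.
; CheckCollision tests overlap only against player character 0 and passes the hitbox damage to its TakeDamage, regardless of hitbox type.
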(event Custom|SpawnHitbox
  (switch Utilities|FlowControl|Switch|SwitchonEHitboxEnum (Variables|Default|GethitboxType)
    (:HB_PROXIMITY
      (Rendering|Material|SetMaterial (Variables|Default|GetHitboxDisplay) 0 "/Game/Art/Materials/Hitboxes/M_ProximityHitbox.M_ProximityHitbox"))
    (:HB_STRIKE
      (Rendering|Material|SetMaterial (Variables|Default|GetHitboxDisplay) 0 "/Game/Art/Materials/Hitboxes/M_StrikeHitbox.M_StrikeHitbox"))
    (:HB_HURTBOX
      (Rendering|Material|SetMaterial (Variables|Default|GetHitboxDisplay) 0 "/Game/Art/Materials/Hitboxes/M_Hurtbox.M_Hurtbox")))
  (Transformation|SetWorldLocation (Variables|Default|GetHitboxDisplay) (Variables|Default|GethitboxLocation) false false)
  (Rendering|SetVisibility (Variables|Default|GetHitboxDisplay) true false))

(event Custom|CheckCollision
  (bind _returnvalue (Game|GetPlayerCharacter 0))
  (if (Collision|IsOverlappingActor _returnvalue :!class /Script/Engine.Actor)
    (bind _asstri_ve_character (Utilities|Casting|CastTostriVeCharacter _returnvalue))
    (Class|StriVeCharacter|TakeDamage _asstri_ve_character (Variables|Default|GethitboxDamage))))

(fn ConstructionScript)