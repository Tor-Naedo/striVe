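; Game mode that sets up a two-character versus match from the players' selected character classes.
; On BeginPlay it spawns each character at PlayerStarts tagged P1 and P2, choosing the class from per-player selections in BaseGameInstance.
; Player controller 0 possesses P1, while P2 gets a directly spawned BasePlayerController.
; With both valid, it cross-links them as opponents, flips P2 and displays the health widget.
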(event EventBeginPlay
  (bind _player1 (Variables|Default|Getplayer1))
  (bind _player2 (Variables|Default|Getplayer2))
  (bind _outactors (Actor|GetAllActorsOfClass "/Script/Engine.PlayerStart"))
  (for _array_element _outactors
    (CallFunction|SpawnPlayers _array_element))
  (if (Utilities|IsValid (Variables|Default|Getplayer1))
    (if (Utilities|IsValid (Variables|Default|Getplayer2))
      (Variables|/Script/striVe.striVeCharacter|SetotherPlayer _player1 _player2)
      (Variables|/Script/striVe.striVeCharacter|SetotherPlayer _player2 _player1)
      (Variables|/Script/striVe.striVeCharacter|SetisFlipped _player2 true)
      (bind _returnvalue (UserInterface|CreateWidget "/Game/UI/WB_Health.WB_Health_C" (Game|GetPlayerController 0)))
      (UserInterface|Viewport|AddtoViewport _returnvalue 0))))

(fn ConstructionScript)

(fn SpawnPlayers
  (params (Object :type Actor%20Object%20Reference))
  (bind _returnvalue (Transformation|GetActorTransform Object))
  (bind _asplayer_start (Utilities|Casting|CastToPlayerStart Object))
  (if (Utilities|Name|Equal(Name) "P1" (Variables|/Script/Engine.PlayerStart|GetPlayerStartTag _asplayer_start))
    (bind _characterreference (CallFunction|DetermineCharacterClass (Transformation|GetActorTransform Object) Object))
    (Variables|Default|Setplayer1 _characterreference)
    (Pawn|Possess (Game|GetPlayerController 0) _characterreference)
    (elif (Utilities|Name|Equal(Name) (Variables|/Script/Engine.PlayerStart|GetPlayerStartTag _asplayer_start) "P2")
      (bind _returnvalue_2 (Game|SpawnActorfromClass "/Script/striVe.BasePlayerController" _returnvalue "Undefined" 0 0))
      (bind _characterreference_2 (CallFunction|DetermineCharacterClass _returnvalue Object 1))
      (Variables|Default|Setplayer2 _characterreference_2)
      (Pawn|Possess _returnvalue_2 _characterreference_2))))

(fn DetermineCharacterClass
  (params (Transform :type Transform) (Actor :type Actor%20Object%20Reference) (PlayerIndex :type Integer))
  (bind _asbase_game_instance (Utilities|Casting|CastToBaseGameInstance (Game|GetGameInstance)))
  (switch int PlayerIndex
    (:Default
      (switch Utilities|FlowControl|Switch|SwitchonECharacterClass (Variables|/Script/striVe.BaseGameInstance|GetP1CharacterClass _asbase_game_instance) :!label _label
        (:VE_Default
          _)
        (:VE_FastCharacter
          (bind _returnvalue (Game|SpawnActorfromClass "/Game/Character/Chara/FastCharacterBP.FastCharacterBP_C" Transform "Undefined" Actor 0 :!label _label_2))
          (return _returnvalue))
        (:VE_StrongCharacter
          (bind _returnvalue_2 (Game|SpawnActorfromClass "/Game/Character/Chara/StrongCharacterBP.StrongCharacterBP_C" Transform "Undefined" Actor 0 :!label _label_3))
          (return _returnvalue_2))
        (:VE_GrapplerCharacter
          (bind _returnvalue_3 (Game|SpawnActorfromClass "/Game/Character/Chara/GrapplerBP.GrapplerBP_C" Transform "Undefined" Actor 0 :!label _label_4))
          (return _returnvalue_3))))
    (:0
      (goto _label))
    (:1
      (switch Utilities|FlowControl|Switch|SwitchonECharacterClass (Variables|/Script/striVe.BaseGameInstance|GetP2CharacterClass _asbase_game_instance)
        (:VE_Default
          _)
        (:VE_FastCharacter
          (goto _label_2))
        (:VE_StrongCharacter
          (goto _label_3))
        (:VE_GrapplerCharacter
          (goto _label_4)))))
  (bind _returnvalue_4 (Game|SpawnActorfromClass "/Game/Character/Chara/BaseCharacterBP.BaseCharacterBP_C" Transform "Undefined" Actor 0))
  (return _returnvalue_4))